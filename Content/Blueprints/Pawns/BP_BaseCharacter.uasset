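; Base player character that handles grab, pick, release/place and punch input and owns the HUD and menu widgets.
; Input sets state flags: grab lasts while held, while the other actions pulse briefly through delays.
; Tick retries setup of the Hiter, Grabber and Picker components until all report ready.
; Events show or hide the menu and update GUI items, and GetActorType selects broken or regular block classes.
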(event EventBActiveMenu
  (params (bIsMenuActive :type Boolean))
  (if bIsMenuActive
    (bind _returnvalue (UserInterface|CreateWidget "/Game/Blueprints/General/BP_Menu.BP_Menu_C"))
    (UserInterface|Viewport|AddtoViewport _returnvalue 0)
    (else
      (Widget|RemovefromParent _returnvalue))))

(event EventAddtoGUI
  (params (ID :type Integer))
  (Default|ChangeItem (stale EventConfigurateBlueprints _returnvalue) ID))

(event EventConfigurateBlueprints
  (bind _returnvalue (UserInterface|CreateWidget "/Game/Blueprints/General/BP_GUI.BP_GUI_C"))
  (UserInterface|Viewport|AddtoViewport _returnvalue 0))

(event EventTick
  (params (DeltaSeconds :type Float%20%28single-precision%29))
  (bind _grabber (Variables|Default|GetGrabber))
  (bind _picker (Variables|Default|GetPicker))
  (bind _hiter (Variables|Default|GetHiter))
  (if (not (Math|Boolean|ANDBoolean (Variables|/Script/CubeCraft2_0.Hiter|GetIsSetHiter _hiter) (Variables|/Script/CubeCraft2_0.Grabber|GetIsSetGrabber _grabber) (Variables|/Script/CubeCraft2_0.Picker|GetIsSetPicker _picker)))
    (Class|Hiter|SetUpInputComponent _hiter)
    (Class|Grabber|SetUpInputComponent _grabber)
    (Class|Grabber|FindPhysicsHandle _grabber)
    (Class|Picker|SetUpInputComponent _picker)))

(event Input|ActionEvents|InputActionGrab
  (params (Key :type Key%20Structure :default "None"))
  (:Pressed
    (Variables|Default|SetisGrabbing true))
  (:Released
    (Variables|Default|SetisGrabbing false)))

(event Input|ActionEvents|InputActionPick
  (params (Key :type Key%20Structure :default "None"))
  (:Pressed
    (Variables|Default|SetisPicking true)
    (Utilities|FlowControl|Delay 0.5)
    (Variables|Default|SetisPicking false)))

(event Input|ActionEvents|InputActionPunch
  (params (Key :type Key%20Structure :default "None"))
  (:Pressed
    (Variables|Default|SetisPunching true)
    (Utilities|FlowControl|Delay 0.5)
    (Variables|Default|SetisPunching false)))

(event Input|ActionEvents|InputActionRelease
  (params (Key :type Key%20Structure :default "None"))
  (:Pressed
    (Variables|Default|SetisReleasing true)
    (Utilities|FlowControl|Delay 0.5)
    (Variables|Default|SetisReleasing false)))

(event Input|ActionEvents|InputActionPlace
  (params (Key :type Key%20Structure :default "None"))
  (:Pressed
    (Variables|Default|SetisReleasing true)
    (Utilities|FlowControl|Delay 0.5)
    (Variables|Default|SetisReleasing false)))

(fn ConstructionScript)

(fn GetActorType
  (params (Type :type Integer))
  (if (Math|Conversions|ToBoolean(Integer) Type)
    (return "/Game/Blueprints/General/BP_BrokenBlock.BP_BrokenBlock_C")
    (else
      (return "/Game/Blueprints/General/BP_Block.BP_Block_C"))))