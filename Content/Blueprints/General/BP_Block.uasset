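; BP_Block is a block actor whose look is driven by an ID that selects the material on its base mesh.
; On BeginPlay it applies the material for a positive ID, or otherwise picks a random ID from the material count.
; SetMesh changes the ID and material, and ScratchMaterial swaps in that ID's scratched variant.
; GetMesh returns the ID despite its name, and GetBlockType returns BP_BrokenBlock.
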(event EventScratchMaterial
  ;[1 1 1] Scratch
  (bind _returnvalue (CallFunction|GetScratchedMaterial (Variables|Default|GetID)))
  (Rendering|Material|SetMaterial (Variables|Default|GetBaseMesh) 0 _returnvalue))

(event EventSetMesh
  (params (id :type Integer))
  ;[1 1 1] SetMaterial
  (Variables|Default|SetID id)
  (bind _returnvalue (CallFunction|GetMaterial id))
  (Rendering|Material|SetMaterial (Variables|Default|GetBaseMesh) 0 _returnvalue))

(event EventBeginPlay
  ;[1 1 1] OnStart RandMaterial
  (if (> (Variables|Default|GetID) 0)
    (bind _returnvalue (CallFunction|GetMaterial (Variables|Default|GetID)))
    (Rendering|Material|SetMaterial (Variables|Default|GetBaseMesh) 0 _returnvalue)
    (else
      (bind _materialcount1 (CallFunction|GetMaterialCount))
      (bind _result (Math|Integer|IncrementInt (Math|Random|RandomInteger _materialcount1))
        (:%20%20
          (bind _output_get (Variables|Default|SetID _result))
          (bind _returnvalue_2 (CallFunction|GetMaterial _output_get))
          (Rendering|Material|SetMaterial (Variables|Default|GetBaseMesh) 0 _returnvalue_2))))))

(fn ConstructionScript)

(fn GetMesh
  (return (Variables|Default|GetID)))

(fn GetBlockType
  (return "/Game/Blueprints/General/BP_BrokenBlock.BP_BrokenBlock_C"))